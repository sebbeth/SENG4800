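; Spline-following train actor that serves as either the locomotive or, via IsWagon, a colored coal hopper wagon.
; Construction estimates its start distance on DrivingRail's spline from sampled points near the actor.
; Each tick, the locomotive advances by clamped CurrentSpeed, while wagons docked through box overlaps hold a fixed offset from their neighbor.
; Two bogies follow the wrapping spline and position the body between them, with roll from yaw change in curves.
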(event `self.ReceiveBeginPlay`
  (bind _returnvalue (`SceneComponent.K2_GetComponentLocation` (`self.Bogie_Front`)))
  (bind _returnvalue_2 (* (+ _returnvalue (`SceneComponent.K2_GetComponentLocation` (`self.Bogie_Back`))) 0.5))
  (bind (_returnvalue_roll _returnvalue_pitch _returnvalue_yaw) (`KismetMathLibrary.BreakRotator` (`KismetMathLibrary.FindLookAtRotation` _returnvalue_2 _returnvalue)))
  (`Timeline|Timeline_0`
    (:`Update`
      (`|ExecutionSequence`
        (:`then_0`
          (`self.Update_Bogie_Movement`))
        (:`then_1`
          ;[1 1 1] Update Body Rotation
          (`SceneComponent.K2_SetWorldTransform` (`self.TrainBody`) (`KismetMathLibrary.MakeTransform` (+ _returnvalue_2 (`KismetMathLibrary.MakeVector` 0.0 0.0 (`self.Train_Z_Offset`))) (`KismetMathLibrary.MakeRotator` _returnvalue_roll _returnvalue_pitch _returnvalue_yaw)) false false))))))

(event `self.ReceiveTick`
  (params (DeltaSeconds :type "Float (single-precision)"))
  (bind _docked_back (`self.Docked_Back`))
  (bind _docked_front (`self.Docked_Front`))
  (bind _max_speed (`self.Max_Speed`))
  (`|ExecutionSequence`
    (:`then_0`
      ;[1 1 1] Move_If_Docked
      (set `self.Delta_Time` DeltaSeconds)
      (if (`self.IsWagon`)
        (`/Engine/EditorBlueprintResources/StandardMacros.IsValid` _docked_back
          (:`Is Valid`
            (set `self.Distance_Along_Rail` (+ (`/Game/Blueprints/BP_Train.Distance_Along_Rail` _docked_back) -740.0))
            (`|ExecutionSequence`
              (:`then_0`
                (`self.Update_Bogie_Movement`))
              (:`then_1`
                (`self.Update_Train_Body`))))
          (:`Is Not Valid`
            (`/Engine/EditorBlueprintResources/StandardMacros.IsValid` _docked_front
              (:`Is Valid`
                (set `self.Distance_Along_Rail` (+ (`/Game/Blueprints/BP_Train.Distance_Along_Rail` _docked_front) 740.0))
                (`|ExecutionSequence`
                  (:`then_0`
                    (`self.Update_Bogie_Movement`))
                  (:`then_1`
                    (`self.Update_Train_Body`)))))))))
    (:`then_1`
      ;[1 1 1] PlayerInput
      (if (not (`self.IsWagon`))
        (bind _output_get (set `self.Current_Speed` (`KismetMathLibrary.FClamp` (`self.Current_Speed`) (* _max_speed -1.0) _max_speed)))
        (`|ExecutionSequence`
          (:`then_0`
            (set `self.Distance_Along_Rail` (+ (`self.Current_Speed`) (`self.Distance_Along_Rail`)))
            (`self.Update_Bogie_Movement`))
          (:`then_1`
            (`self.Update_Train_Body`)))))))

(event `self.Box_Back.OnComponentBeginOverlap`
  (params (OverlappedComponent :type "PrimitiveComponent Object Reference") (OtherActor :type "Actor Object Reference") (OtherComp :type "PrimitiveComponent Object Reference") (OtherBodyIndex :type Integer) (bFromSweep :type Boolean) (SweepResult :type "HitResult Structure (by ref)"))
  ;[1 1 1] Wagon Docking (Needs Work)
  (bind _asbp_train (cast `/Game/Blueprints/BP_Train` OtherActor))
  (if (not (`/Game/Blueprints/BP_Train.Docked_To_Train` _asbp_train))
    (`/Engine/EditorBlueprintResources/StandardMacros.DoOnce` false
      (:`Completed`
        (`self.Event_Attach_Back` _asbp_train self)))))

(event `Event_Attach_Back`
  (params (Wagon :type "/Game/Blueprints/BP_Train Object Reference"))
  ;[1 1 1] Wagon Docking (Needs Work)
  (set `self.Docked_Back` Wagon)
  (set `self.Docked_To_Train` true))

(event `self.Box_Front.OnComponentBeginOverlap`
  (params (OverlappedComponent :type "PrimitiveComponent Object Reference") (OtherActor :type "Actor Object Reference") (OtherComp :type "PrimitiveComponent Object Reference") (OtherBodyIndex :type Integer) (bFromSweep :type Boolean) (SweepResult :type "HitResult Structure (by ref)"))
  ;[1 1 1] Wagon Docking (Needs Work)
  (bind _asbp_train (cast `/Game/Blueprints/BP_Train` OtherActor))
  (if (not (`/Game/Blueprints/BP_Train.Docked_To_Train` _asbp_train))
    (`/Engine/EditorBlueprintResources/StandardMacros.DoOnce` false
      (:`Completed`
        (`self.Event_Attach_Front` _asbp_train self)))))

(event `Event_Attach_Front`
  (params (Wagon :type "/Game/Blueprints/BP_Train Object Reference"))
  ;[1 1 1] Wagon Docking (Needs Work)
  (set `self.Docked_Front` Wagon)
  (set `self.Docked_To_Train` true))

(fn `Update_Train_Body`
  (locals (RotationMultiplier :type "Float (double-precision)"))
  (bind _returnvalue (`SceneComponent.K2_GetComponentLocation` (`self.Bogie_Front`)))
  (bind _returnvalue_2 (* (+ _returnvalue (`SceneComponent.K2_GetComponentLocation` (`self.Bogie_Back`))) 0.5))
  (bind (_returnvalue_roll _returnvalue_pitch _returnvalue_yaw) (`KismetMathLibrary.BreakRotator` (`KismetMathLibrary.FindLookAtRotation` _returnvalue_2 _returnvalue)))
  (`|ExecutionSequence`
    (:`then_0`
      ;[1 1 1] Check If Train Moves Forward or Backward (Necassary for Train Rotation while driving curves)
      (if (>= (`self.Current_Speed`) 0.0)
        (set `local.RotationMultiplier` 1.0)
        (else
          (set `local.RotationMultiplier` -1.0))))
    (:`then_1`
      ;[1 1 1] Update Body Rotation
      (`SceneComponent.K2_SetWorldTransform` (`self.TrainBody`) (`KismetMathLibrary.MakeTransform` (+ _returnvalue_2 (`KismetMathLibrary.MakeVector` 0.0 0.0 (`self.Train_Z_Offset`))) (`KismetMathLibrary.MakeRotator` (+ _returnvalue_roll (* (- (`self.Last_Z_Rot`) _returnvalue_yaw) -10.0 (`local.RotationMultiplier`))) _returnvalue_pitch _returnvalue_yaw)) false false)
      (set `self.Last_Z_Rot` _returnvalue_yaw))))

(fn `UserConstructionScript`
  (locals (Last_Vector_Lenght :type "Float (double-precision)" :default 100000.0))
  (bind _trainbody (`self.TrainBody`))
  (bind _relativelocation_x (`KismetMathLibrary.BreakVector` (`SceneComponent.RelativeLocation` (`self.Bogie_Back`))))
  (bind _ingame_spline (`/Game/Blueprints/BP_Rails.Ingame_Spline` (`self.DrivingRail`)))
  (bind _relativelocation_x_2 (`KismetMathLibrary.BreakVector` (`SceneComponent.RelativeLocation` (`self.Bogie_Front`))))
  (bind _returnvalue (- (`SplineComponent.GetNumberOfSplinePoints` _ingame_spline) 4))
  (`|ExecutionSequence`
    (:`then_0`
      ;[1 1 1] Position Train/Wagon on closest Spline
      (for _index (range 1 (+ _returnvalue 1))
        (if (== (mod _index (/ _returnvalue 200)) 0)
          (bind _returnvalue_2 (`KismetMathLibrary.VSize` (- (`SplineComponent.FindLocationClosestToWorldLocation` _ingame_spline (`self.K2_GetActorLocation`) "World") (`SplineComponent.GetLocationAtSplinePoint` _ingame_spline _index "World"))))
          (if (< _returnvalue_2 (`local.Last_Vector_Lenght`))
            (set `local.Last_Vector_Lenght` _returnvalue_2)
            (set `self.Start_Distance` (`SplineComponent.GetDistanceAlongSplineAtSplinePoint` _ingame_spline _index))
            (`self.K2_SetActorRotation` self (`SplineComponent.GetRotationAtSplinePoint` _ingame_spline _index "World") false)))))
    (:`then_1`
      ;[1 1 1] Set_Values
      (bind _output_get (set `self.BogieDistance` (+ (`KismetMathLibrary.Abs` _relativelocation_x_2) (`KismetMathLibrary.Abs` _relativelocation_x))))
      (set `self.Distance_Along_Rail` (+ (* _output_get 0.5) (`self.Start_Distance`)))
      ;[1 1 1] Check If Is Wagon
      (if (`self.IsWagon`)
        (`StaticMeshComponent.SetStaticMesh` _trainbody "/Game/Geometry/CoalHopper/CoalHopperFull.CoalHopperFull")
        (bind _returnvalue_3 (`PrimitiveComponent.CreateDynamicMaterialInstance` _trainbody 0 "/Game/Geometry/CoalHopper/Coal.Coal"))
        (`MaterialInstanceDynamic.SetVectorParameterValue` _returnvalue_3 "CustomColorSwitch" (`self.Color`))))))