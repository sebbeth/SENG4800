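; Stacker-reclaimer machine actor that shows its operating state by material and can rotate its tower.
; Custom events swap the first material slot of the static mesh between stacking, reclaiming and default loader-yellow materials.
; SetRotation converts its input to float and applies it as the Tower component's relative yaw, zeroing pitch and roll.
; It has no Tick or construction logic, so changes happen only when these events are called.
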(event `self.ReceiveTick`
  (params (DeltaSeconds :type "Float (single-precision)")))

(event `self.ReclaimMaterial`
  (`PrimitiveComponent.SetMaterial` (`self.StaticMesh`) 0 "/Game/Materials/SR_Reclaiming.SR_Reclaiming"))

(event `self.ResetMaterial`
  (`PrimitiveComponent.SetMaterial` (`self.StaticMesh`) 0 "/Game/Geometry/Loader/Loader_yellow.Loader_yellow"))

(event `self.StackMaterial`
  (`PrimitiveComponent.SetMaterial` (`self.StaticMesh`) 0 "/Game/Materials/SR_Stacking.SR_Stacking"))

(event `self.setRotation`
  (params (rotation :type Integer))
  (`SceneComponent.K2_SetRelativeRotation` (`self.Tower`) (`KismetMathLibrary.MakeRotator` 0.0 0.0 (`KismetMathLibrary.Conv_IntToDouble` rotation)) false false))

(fn `UserConstructionScript`)